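; Openable door actor that swings about its yaw axis when its OpenDoor member fires open and close events.
; It stores its starting rotation on BeginPlay, then the DoorSwing timeline adds an animated angle to that yaw each update.
; Opening plays the timeline and closing reverses it.
; An event track on the timeline times the lock sound at the door's location.
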(event `self.ReceiveBeginPlay`
  (bind _output_get (set `self.BeginAngle` (`self.K2_GetActorRotation`))))

(event `self.OpenDoor.OnOpen`
  (bind (_direction _openangle) (`Timeline|DoorSwing` :!label _label)
    (:`Update`
      (`self.K2_SetActorRotation` (`KismetMathLibrary.MakeRotator` (.roll (stale `self.ReceiveBeginPlay` _output_get)) (.pitch (stale `self.ReceiveBeginPlay` _output_get)) (+ (.yaw (stale `self.ReceiveBeginPlay` _output_get)) (.yaw (`KismetMathLibrary.MakeRotator` 0.0 0.0 _openangle))))))
    (:`SoundTiming`
      (`GameplayStatics.PlaySoundAtLocation` "/Game/Audio/door-lock.door-lock" (`self.K2_GetActorLocation`)))))

(event `self.OpenDoor.OnClose`
  (goto _label :!via `Reverse`))

(fn `UserConstructionScript`)